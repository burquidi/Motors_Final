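; KeySpawnerBP is a pressure button that spawns a collectible key when the player character IcaroBP steps on it.
; An overlap on its Box plays a timeline that offsets the button mesh vertically from its starting position.
; When the timeline finishes, the button is flagged as down, so later overlaps are ignored, and a CollectibleKeysBP spawns at the SpawnLocation component's transform.
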(event OnComponentBeginOverlap(Box)
  (params (OverlappedComponent :type Primitive%20Component%20Object%20Reference) (OtherActor :type Actor%20Object%20Reference) (OtherComp :type Primitive%20Component%20Object%20Reference) (OtherBodyIndex :type Integer) (bFromSweep :type Boolean) (SweepResult :type Hit%20Result%20Structure%20%28by%20ref%29))
  (Utilities|Casting|CastToIcaroBP OtherActor)
  (if (not (Variables|Default|GetisDown))
    (bind _value (Timeline|Timeline_0 Play)
      (:Update
        (Transformation|SetRelativeLocation (Variables|Default|GetButtonSM) (+ (Math|Vector|MakeVector 0.0 0.0 _value) (Variables|Default|GetbuttonInitialPosition)) false false))
      (:Finished
        (Variables|Default|SetisDown true)
        (Game|SpawnActorfromClass "/Game/Blueprints/Collectibles/CollectibleKeysBP.CollectibleKeysBP_C" (Transformation|GetWorldTransform (Variables|Default|GetSpawnLocation)) "Undefined" 0 0)))))

(event EventBeginPlay
  (Variables|Default|SetbuttonInitialPosition (Variables|/Script/Engine.SceneComponent|GetRelativeLocation (Variables|Default|GetButtonSM))))

(event Collision|EventActorBeginOverlap
  (params (OtherActor :type Actor%20Object%20Reference)))

(event EventTick
  (params (DeltaSeconds :type Float%20%28single-precision%29)))

(fn ConstructionScript)