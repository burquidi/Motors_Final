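; Locked door that the IcaroBP character opens by spending one of its keys on overlap.
; Front and back box triggers each check the key count and that the door is still closed, then call KeysDown and play their own timeline.
; The timelines lerp the whole actor's rotation from the mesh's initial relative rotation to opposite 110-degree angles, setting IsOpen, with no logic to close it.
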(event OnComponentBeginOverlap(BoxFront)
  (params (OverlappedComponent :type Primitive%20Component%20Object%20Reference) (OtherActor :type Actor%20Object%20Reference) (OtherComp :type Primitive%20Component%20Object%20Reference) (OtherBodyIndex :type Integer) (bFromSweep :type Boolean) (SweepResult :type Hit%20Result%20Structure%20%28by%20ref%29))
  (bind _asicaro_bp (Utilities|Casting|CastToIcaroBP OtherActor))
  (if (>= (Variables|/Game/Blueprints/IcaroBP.IcaroBP_C|GetKeys _asicaro_bp) 1)
    (if (not (Variables|Default|GetisOpen))
      (Default|KeysDown _asicaro_bp)
      (bind _value (Timeline|Timeline_0 Play)
        (:Update
          (Transformation|SetActorRotation (Math|Rotator|Lerp(Rotator) (Variables|Default|GetInitialRotation) "0.000000,-110.000000, 0" _value true))
          (Variables|Default|SetisOpen true))))))

(event OnComponentBeginOverlap(BoxBack)
  (params (OverlappedComponent :type Primitive%20Component%20Object%20Reference) (OtherActor :type Actor%20Object%20Reference) (OtherComp :type Primitive%20Component%20Object%20Reference) (OtherBodyIndex :type Integer) (bFromSweep :type Boolean) (SweepResult :type Hit%20Result%20Structure%20%28by%20ref%29))
  (bind _asicaro_bp (Utilities|Casting|CastToIcaroBP OtherActor))
  (if (>= (Variables|/Game/Blueprints/IcaroBP.IcaroBP_C|GetKeys _asicaro_bp) 1)
    (if (not (Variables|Default|GetisOpen))
      (Default|KeysDown _asicaro_bp)
      (bind _value (Timeline|Timeline_1 Play)
        (:Update
          (Transformation|SetActorRotation (Math|Rotator|Lerp(Rotator) (Variables|Default|GetInitialRotation) "0.000000,110.000000, 0" _value true))
          (Variables|Default|SetisOpen true))))))

(event EventBeginPlay
  (Variables|Default|SetInitialRotation (Variables|/Script/Engine.SceneComponent|GetRelativeRotation (Variables|Default|GetDoorSM)))
  (Variables|Default|SetisOpen false))

(event Collision|EventActorBeginOverlap
  (params (OtherActor :type Actor%20Object%20Reference)))

(event EventTick
  (params (DeltaSeconds :type Float%20%28single-precision%29)))

(fn ConstructionScript)