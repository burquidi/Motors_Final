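; StoneDoorBP is a stone door that slides open when the Icaro character (IcaroBP) enters the trigger box in front of it.
; The front box overlap plays a timeline that offsets the door mesh along local Y from the position cached at BeginPlay.
; An IsOpen flag, set as the timeline updates, blocks retriggering, and the graph has no logic to close the door.
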(event OnComponentBeginOverlap(BoxFront)
  (params (OverlappedComponent :type Primitive%20Component%20Object%20Reference) (OtherActor :type Actor%20Object%20Reference) (OtherComp :type Primitive%20Component%20Object%20Reference) (OtherBodyIndex :type Integer) (bFromSweep :type Boolean) (SweepResult :type Hit%20Result%20Structure%20%28by%20ref%29))
  (Utilities|Casting|CastToIcaroBP OtherActor)
  (if (not (Variables|Default|GetisOpen))
    (bind _value (Timeline|Timeline_0 Play)
      (:Update
        (Transformation|SetRelativeLocation (Variables|Default|GetDoorSM) (+ (Math|Vector|MakeVector 0.0 _value 0.0) (Variables|Default|GetInitialPosition)) false false)
        (Variables|Default|SetisOpen true)))))

(event EventBeginPlay
  (Variables|Default|SetInitialPosition (Variables|/Script/Engine.SceneComponent|GetRelativeLocation (Variables|Default|GetDoorSM)))
  (Variables|Default|SetisOpen false))

(event Collision|EventActorBeginOverlap
  (params (OtherActor :type Actor%20Object%20Reference)))

(event EventTick
  (params (DeltaSeconds :type Float%20%28single-precision%29)))

(fn ConstructionScript)