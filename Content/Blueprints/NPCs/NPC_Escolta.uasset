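; NPC_Escolta is an NPC Blueprint that gives its mesh a random color each time play begins.
; The construction script creates a dynamic material instance from MAT6_2_Inst, stores it and assigns it to the first material slot of Mesh.
; BeginPlay then sets that instance's BaseColor parameter from random red, green and blue values, so each spawned NPC gets its own tint.
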(event EventBeginPlay
  (Rendering|Material|SetVectorParameterValue (Variables|Default|GetMaterial) "BaseColor" (Math|Color|MakeColor (Math|Random|RandomFloatinRange 0.0 1.0) (Math|Random|RandomFloatinRange 0.0 1.0) (Math|Random|RandomFloatinRange 0.0 1.0)) :!class /Script/Engine.MaterialInstanceDynamic))

(fn ConstructionScript
  (bind _returnvalue (Rendering|Material|CreateDynamicMaterialInstance "/Game/Blueprints/Materials/MAT6_2_Inst.MAT6_2_Inst" :!class /Script/Engine.KismetMaterialLibrary))
  (bind _output_get (Variables|Default|SetMaterial _returnvalue))
  (Rendering|Material|SetMaterial (Variables|Character|GetMesh) 0 _output_get))