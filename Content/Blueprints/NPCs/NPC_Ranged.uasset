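; NPC_Ranged is an enemy NPC Blueprint that tracks its own health and damages the IcaroBP player character on capsule hits.
; NPCHPDown subtracts a fixed amount of health and clamps at zero, with no death handling.
; GiveExperience, not called within this Blueprint, adds experience to the player and handles level-ups by resetting experience and doubling the threshold.
; Despite the name, no ranged attack logic appears here.
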(event OnComponentHit(CapsuleComponent)
  (params (HitComponent :type Primitive%20Component%20Object%20Reference) (OtherActor :type Actor%20Object%20Reference) (OtherComp :type Primitive%20Component%20Object%20Reference) (NormalImpulse :type Vector :default "0, 0, 0") (Hit :type Hit%20Result%20Structure%20%28by%20ref%29))
  (bind _asicaro_bp (Utilities|Casting|CastToIcaroBP OtherActor))
  (Default|HPDown _asicaro_bp))

(event EventBeginPlay
  (Variables|Default|SetNPCHealth (Variables|Default|GetNPCMaxNPC)))

(fn ConstructionScript)

(fn GiveExperience
  (bind _asicaro_bp (Utilities|Casting|CastToIcaroBP (Game|GetPlayerCharacter 0)))
  (bind _output_get (Variables|/Game/Blueprints/IcaroBP.IcaroBP_C|SetExperience _asicaro_bp (+ (Variables|/Game/Blueprints/IcaroBP.IcaroBP_C|GetExperience _asicaro_bp) (Variables|Default|GetExperienceGiven))))
  (if (>= _output_get (Variables|/Game/Blueprints/IcaroBP.IcaroBP_C|GetMaxExperience _asicaro_bp))
    (bind _result (Math|Integer|IncrementInt (Variables|/Game/Blueprints/IcaroBP.IcaroBP_C|GetLevel _asicaro_bp))
      (:%20%20
        (Variables|/Game/Blueprints/IcaroBP.IcaroBP_C|SetLevel _asicaro_bp _result)
        (Variables|/Game/Blueprints/IcaroBP.IcaroBP_C|SetExperience _asicaro_bp 0)
        (Variables|/Game/Blueprints/IcaroBP.IcaroBP_C|SetMaxExperience _asicaro_bp (* (Variables|/Game/Blueprints/IcaroBP.IcaroBP_C|GetMaxExperience _asicaro_bp) 2))))))

(fn NPCHPDown
  (bind _output_get (Variables|Default|SetNPCHealth (- (Variables|Default|GetNPCHealth) 5.0)))
  (if (<= _output_get 0.0)
    (Variables|Default|SetNPCHealth 0.0)))