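; AI controller for an NPC in a group tag ("pilla-pilla") game, driven by a behavior tree.
; On BeginPlay it sets up the BBGrupoPillaPilla blackboard, stores its controlled pawn as "YoMisMo" (itself), and runs the BT_GrupoPillaPilla tree.
; The LaLlevoYo event writes that pawn into "ElQueLaLleva", marking this NPC as the one who is "it".
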(event Custom|LaLlevoYo
  (AI|Components|Blackboard|SetValueasObject (Variables|Default|GetBB) (Utilities|Name|MakeLiteralName "ElQueLaLleva") (Pawn|GetControlledPawn)))

(event EventBeginPlay
  (bind _blackboardcomponent (Class|AIController|UseBlackboard "/Game/Blueprints/NPC/BT_GrupoPillaPilla/BBGrupoPillaPilla.BBGrupoPillaPilla"))
  (bind _output_get (Variables|Default|SetBB _blackboardcomponent))
  (AI|Components|Blackboard|SetValueasObject _output_get (Utilities|Name|MakeLiteralName "YoMisMo") (Pawn|GetControlledPawn))
  (AI|RunBehaviorTree "/Game/Blueprints/NPC/BT_GrupoPillaPilla/BT_GrupoPillaPilla.BT_GrupoPillaPilla"))

(fn ConstructionScript)