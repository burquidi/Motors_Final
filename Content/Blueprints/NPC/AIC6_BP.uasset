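; AI controller for zombie NPCs that runs the BT_Zombies behavior tree on the BB_AZ blackboard.
; On BeginPlay it stores its pawn under "Me" and creates a ZombiesArray object in the shared "Zombies" key if no other controller has done so.
; The LaLlevoYo event adds the controlled pawn to that array, so the controllers share one list of zombies through the blackboard.
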(event Custom|LaLlevoYo
  (Utilities|Set|Add (Variables|/Game/Blueprints/NPC/BT_Zombies/ZombiesArray.ZombiesArray_C|GetZombies (.AsZombies%20Array (Utilities|Casting|CastToZombiesArray (AI|Components|Blackboard|GetValueasObject (Variables|Default|GetBB) (Utilities|Name|MakeLiteralName "Zombies"))))) (Pawn|GetControlledPawn)))

(event EventBeginPlay
  ;[1 1 1] Le indico que blackboard utilizar y guardo una referencia a ésta en BB
  (bind _blackboardcomponent (Class|AIController|UseBlackboard "/Game/Blueprints/NPC/BT_Zombies/BB_AZ.BB_AZ"))
  (bind _output_get (Variables|Default|SetBB _blackboardcomponent))
  (AI|Components|Blackboard|SetValueasObject _output_get (Utilities|Name|MakeLiteralName "Me") (Pawn|GetControlledPawn))
  ;[1 1 1] Compruebo si el objeto compartido ZombiesArray ya ha sido instanciado por otro controlador
  (if (== (AI|Components|Blackboard|GetValueasObject (Variables|Default|GetBB) (Utilities|Name|MakeLiteralName "Zombies")) 0)
    ;[1 1 1] Si no, lo instancio y lo guardo en la variable compartida Zombies
    (bind _returnvalue (Game|ConstructObjectfromClass "/Game/Blueprints/NPC/BT_Zombies/ZombiesArray.ZombiesArray_C" self))
    (AI|Components|Blackboard|SetValueasObject (Variables|Default|GetBB) (Utilities|Name|MakeLiteralName "Zombies") _returnvalue))
  (AI|RunBehaviorTree "/Game/Blueprints/NPC/BT_Zombies/BT_Zombies.BT_Zombies"))

(fn ConstructionScript)