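; NPC4 is an NPC with a tagged-style on/off state, toggled by LaLlevoYo ("I'm it") and NoLaLlevoYo ("I'm not it").
; The construction script puts a dynamic material on the mesh, and BeginPlay gives it a random base color.
; Becoming "it" raises the Brillo glow parameter and enables ragdoll physics from spine_03 down the bone chain.
; Losing that state clears the glow and stops all body simulation.
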(event Custom|LaLlevoYo
  (Rendering|Material|SetScalarParameterValue (Variables|Default|GetDynMaterial) "Brillo" 5.0 :!class /Script/Engine.MaterialInstanceDynamic)
  (Class|SkeletalMeshComponent|SetAllBodiesBelowSimulatePhysics (Variables|Character|GetMesh) (Utilities|Name|MakeLiteralName "spine_03") true true))

(event Custom|NoLaLlevoYo
  (Rendering|Material|SetScalarParameterValue (Variables|Default|GetDynMaterial) "Brillo" 0.0 :!class /Script/Engine.MaterialInstanceDynamic)
  (Class|SkeletalMeshComponent|SetAllBodiesSimulatePhysics (Variables|Character|GetMesh) false))

(event EventBeginPlay
  (Rendering|Material|SetVectorParameterValue (Variables|Default|GetDynMaterial) "BaseColor" (Math|Color|MakeColor (Math|Random|RandomFloatinRange 0.0 1.0) (Math|Random|RandomFloatinRange 0.0 1.0) (Math|Random|RandomFloatinRange 0.0 1.0)) :!class /Script/Engine.MaterialInstanceDynamic))

(fn ConstructionScript
  (bind _returnvalue (Rendering|Material|CreateDynamicMaterialInstance "/Game/Blueprints/NPC/MaterialNPC3_Inst.MaterialNPC3_Inst" :!class /Script/Engine.KismetMaterialLibrary))
  (bind _output_get (Variables|Default|SetDynMaterial _returnvalue))
  (Rendering|Material|SetMaterial (Variables|Character|GetMesh) 0 _output_get))