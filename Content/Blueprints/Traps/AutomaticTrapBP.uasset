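; Automatic spike trap that cycles its spikes on a timer and damages the player character IcaroBP.
; Tick toggles a SpikesOut flag through delays, driving a timeline that offsets the spikes' Z from their starting position and reverses after a pause.
; A Box overlap calls HPDown on IcaroBP, with no check of the SpikesOut state.
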(event OnComponentBeginOverlap(Box)
  (params (OverlappedComponent :type Primitive%20Component%20Object%20Reference) (OtherActor :type Actor%20Object%20Reference) (OtherComp :type Primitive%20Component%20Object%20Reference) (OtherBodyIndex :type Integer) (bFromSweep :type Boolean) (SweepResult :type Hit%20Result%20Structure%20%28by%20ref%29))
  (bind _asicaro_bp (Utilities|Casting|CastToIcaroBP OtherActor))
  (Default|HPDown _asicaro_bp))

(event EventBeginPlay
  (Variables|Default|SetstartingPosition (Variables|/Script/Engine.SceneComponent|GetRelativeLocation (Variables|Default|GetSpikes)))
  (Variables|Default|SetspikesOut false))

(event Collision|EventActorBeginOverlap
  (params (OtherActor :type Actor%20Object%20Reference)))

(event EventTick
  (params (DeltaSeconds :type Float%20%28single-precision%29))
  (if (Variables|Default|GetspikesOut)
    (bind _newtrack_0 (Timeline|Timeline_0 Play)
      (:Update
        (Transformation|SetRelativeLocation (Variables|Default|GetSpikes) (+ (Variables|Default|GetstartingPosition) (Math|Vector|MakeVector 0.0 0.0 _newtrack_0)) false false))
      (:Finished
        (Utilities|FlowControl|Delay 3.0)
        (Variables|Default|SetspikesOut false)
        (Timeline|Timeline_0 Reverse)))
    (else
      (Utilities|FlowControl|Delay 3.3)
      (Variables|Default|SetspikesOut true))))

(fn ConstructionScript)