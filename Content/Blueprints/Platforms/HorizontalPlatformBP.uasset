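; Horizontal platform Blueprint that shuttles back and forth along its static mesh's forward vector.
; Each Tick offsets the actor by Speed forward or backward depending on the Proceeding flag, sweeping for collision, with a per-frame step not scaled by delta time.
; It feeds the mesh's world location into SetActorRelativeLocation.
; A Timer accumulates delta seconds and, at a fixed ten-second threshold, flips Proceeding and resets.
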(event EventTick
  (params (DeltaSeconds :type Float%20%28single-precision%29))
  (bind _staticmeshcomponent (Variables|Debug|GetStaticMeshComponent))
  (bind _speed (Variables|Default|Getspeed))
  (bind _returnvalue (Transformation|GetWorldLocation _staticmeshcomponent))
  (bind _returnvalue_2 (Math|Vector|GetForwardVector _staticmeshcomponent))
  (bind _returnvalue_3 (* _returnvalue_2 _speed))
  (if (Variables|Default|Getproceeding)
    (Transformation|SetActorRelativeLocation (+ _returnvalue _returnvalue_3) true)
    (else
      (Transformation|SetActorRelativeLocation (- _returnvalue _returnvalue_3) true)))
  (Math|Float|CompareFloat (Variables|Default|Gettimer) 1e+01
    (:>
      (if (Variables|Default|Getproceeding) :!label _label
        (Variables|Default|Setproceeding false)
        (else
          (Variables|Default|Setproceeding true)))
      (Variables|Default|Settimer 0.0))
    (:==
      (goto _label))
    (:<
      (Variables|Default|Settimer (+ (Variables|Default|Gettimer) DeltaSeconds)))))

(fn ConstructionScript)