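; Platform actor that slides along its forward vector and dissolves away after the player (IcaroBP) first touches its trigger box.
; A timeline started at BeginPlay moves the mesh by an offset from its initial position.
; The first overlap creates a dynamic material whose Amount parameter is animated by a second timeline scaled to DissolveTime, destroying the actor when finished.
; Meanwhile, Tick uses a Delay to print a per-second countdown.
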(event OnComponentBeginOverlap(Box)
  (params (OverlappedComponent :type Primitive%20Component%20Object%20Reference) (OtherActor :type Actor%20Object%20Reference) (OtherComp :type Primitive%20Component%20Object%20Reference) (OtherBodyIndex :type Integer) (bFromSweep :type Boolean) (SweepResult :type Hit%20Result%20Structure%20%28by%20ref%29))
  (Utilities|Casting|CastToIcaroBP OtherActor)
  (Utilities|FlowControl|DoOnce false
    (:Completed
      (bind _returnvalue (Rendering|Material|CreateDynamicMaterialInstance (Variables|Default|GetDissPlatform) 0 "/Game/Blueprints/Platforms/DissolveMaterial_Inst.DissolveMaterial_Inst" :!class /Script/Engine.PrimitiveComponent))
      (Components|Timeline|SetPlayRate (Variables|Default|GetTimeline_1) (/ 1.0 (Variables|Default|GetDissolveTime)))
      (Variables|Default|SetCountDown true)
      (bind _dissolve (Timeline|Timeline_1 Play)
        (:Update
          (Rendering|Material|SetScalarParameterValue _returnvalue "Amount" _dissolve :!class /Script/Engine.MaterialInstanceDynamic))
        (:Finished
          (Actor|DestroyActor))))))

(event OnComponentEndOverlap(Box)
  (params (OverlappedComponent :type Primitive%20Component%20Object%20Reference) (OtherActor :type Actor%20Object%20Reference) (OtherComp :type Primitive%20Component%20Object%20Reference) (OtherBodyIndex :type Integer))
  (Utilities|Casting|CastToIcaroBP OtherActor))

(event Custom|MovementEvt
  (bind _offset (Timeline|Timeline_0 PlayFromStart)
    (:Update
      (Transformation|SetWorldLocation (Variables|Default|GetDissPlatform) (+ (* (Transformation|GetActorForwardVector) (* _offset (Variables|Default|GetOffset))) (Variables|Default|GetInit%20Pos)) false false))))

(event EventBeginPlay
  (Variables|Default|SetInit%20Pos (Transformation|GetActorLocation))
  (CallFunction|MovementEvt)
  (Variables|Default|SetCountDownInt (Math|Float|Truncate (Variables|Default|GetDissolveTime))))

(event EventTick
  (params (DeltaSeconds :type Float%20%28single-precision%29))
  (if (Variables|Default|GetCountDown)
    (Utilities|FlowControl|Delay 1.0)
    (bind _output_get (Variables|Default|SetCountDownInt (- (Variables|Default|GetCountDownInt) 1)))
    (Development|PrintString (Utilities|String|ToString(Integer) _output_get))))

(fn ConstructionScript)