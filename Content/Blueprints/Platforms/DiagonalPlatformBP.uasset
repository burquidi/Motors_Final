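; Moving platform that shuttles back and forth along the diagonal between its mesh's up and forward vectors.
; Each Tick offsets the mesh's world location along that diagonal by Speed, without delta-time scaling, and passes it to a swept SetActorRelativeLocation.
; An accumulated Timer flips the Proceeding flag to reverse direction about every three seconds.
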(event EventTick
  (params (DeltaSeconds :type Float%20%28single-precision%29))
  (bind _staticmeshcomponent (Variables|Debug|GetStaticMeshComponent))
  (bind _speed (Variables|Default|Getspeed))
  (bind _returnvalue (Transformation|GetWorldLocation _staticmeshcomponent))
  (bind _returnvalue_2 (Math|Vector|GetUpVector _staticmeshcomponent))
  (bind _returnvalue_3 (Math|Vector|GetForwardVector _staticmeshcomponent))
  (bind _returnvalue_4 (+ _returnvalue_2 _returnvalue_3))
  (bind _returnvalue_5 (* _returnvalue_4 _speed))
  (if (Variables|Default|Getproceeding)
    (Transformation|SetActorRelativeLocation (+ _returnvalue _returnvalue_5) true)
    (else
      (Transformation|SetActorRelativeLocation (- _returnvalue _returnvalue_5) true)))
  (Math|Float|CompareFloat (Variables|Default|Gettimer) 3.0
    (:>
      (if (Variables|Default|Getproceeding) :!label _label
        (Variables|Default|Setproceeding false)
        (else
          (Variables|Default|Setproceeding true)))
      (Variables|Default|Settimer 0.0))
    (:==
      (goto _label))
    (:<
      (Variables|Default|Settimer (+ (Variables|Default|Gettimer) DeltaSeconds)))))

(fn ConstructionScript)