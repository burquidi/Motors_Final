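; Health pickup collectible that restores HP to the player character when touched.
; On BeginPlay it gives the sphere mesh a dynamic material with a preset dissolve amount.
; When IcaroBP overlaps the sphere, it calls HPUp, then a timeline animates the material's AmountDissolve parameter and the actor destroys itself once the dissolve finishes.
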(event OnComponentBeginOverlap(Sphere)
  (params (OverlappedComponent :type Primitive%20Component%20Object%20Reference) (OtherActor :type Actor%20Object%20Reference) (OtherComp :type Primitive%20Component%20Object%20Reference) (OtherBodyIndex :type Integer) (bFromSweep :type Boolean) (SweepResult :type Hit%20Result%20Structure%20%28by%20ref%29))
  (bind _asicaro_bp (Utilities|Casting|CastToIcaroBP OtherActor))
  (Default|HPUp _asicaro_bp)
  (bind _returnvalue (Rendering|Material|CreateDynamicMaterialInstance (Variables|Default|GetSphereSM) 0 "/Game/MaterialesNuevos/Mat_PickUpVIDA_Inst.Mat_PickUpVIDA_Inst" :!class /Script/Engine.PrimitiveComponent))
  (bind _newtrack_0 (Timeline|Timeline_0 Play)
    (:Update
      (Rendering|Material|SetScalarParameterValue _returnvalue "AmountDissolve" _newtrack_0 :!class /Script/Engine.MaterialInstanceDynamic))
    (:Finished
      (Actor|DestroyActor))))

(event EventBeginPlay
  (bind _returnvalue (Rendering|Material|CreateDynamicMaterialInstance (Variables|Default|GetSphereSM) 0 "/Game/MaterialesNuevos/Mat_PickUpVIDA_Inst.Mat_PickUpVIDA_Inst" :!class /Script/Engine.PrimitiveComponent))
  (Rendering|Material|SetScalarParameterValue _returnvalue "AmountDissolve" -0.2 :!class /Script/Engine.MaterialInstanceDynamic))

(event Collision|EventActorBeginOverlap
  (params (OtherActor :type Actor%20Object%20Reference)))

(event EventTick
  (params (DeltaSeconds :type Float%20%28single-precision%29)))

(fn ConstructionScript)