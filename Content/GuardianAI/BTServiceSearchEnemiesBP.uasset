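; Behavior tree service that searches for targets around the guardian AI's pawn and writes the result to the blackboard.
; Each tick it runs a short, large-radius sphere trace at the pawn, against PhysicsBody objects only, ignoring itself, using a cached guardian controller.
; A hit sets Target and TargetLocation from the single hit actor, with no further enemy filtering.
; A miss clears Target but leaves the last TargetLocation in place.
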(event EventTick
  (params (OwnerActor :type Actor%20Object%20Reference) (DeltaSeconds :type Float%20%28single-precision%29))
  (if (!= (Variables|Default|GetGuardianController) 0)
    _
    (else
      (Variables|Default|SetGuardianController (.AsAIGuardian%20Controller%20BP (Utilities|Casting|CastToAIGuardianControllerBP OwnerActor)))))
  (bind (_outhit _returnvalue) (Collision|SphereTraceForObjects (Transformation|GetActorLocation (Pawn|GetControlledPawn (Variables|Default|GetGuardianController))) (+ (Transformation|GetActorLocation (Pawn|GetControlledPawn (Variables|Default|GetGuardianController))) "0, 0,10.000000") 2.4e+03 (Utilities|Array|MakeArray "ObjectTypeQuery4") false (Utilities|Array|MakeArray (Pawn|GetControlledPawn (Variables|Default|GetGuardianController))) "None"))
  (if _returnvalue
    (Class|BTFunctionLibrary|SetBlackboardValueasObject (Variables|Default|GetTarget) (.HitActor (Collision|BreakHitResult _outhit)))
    (AI|BehaviorTree|SetBlackboardValueasVector (Variables|Default|GetTargetLocation) (Transformation|GetActorLocation (.HitActor (Collision|BreakHitResult _outhit))))
    (else
      (Class|BTFunctionLibrary|ClearBlackboardValue (Variables|Default|GetTarget)))))