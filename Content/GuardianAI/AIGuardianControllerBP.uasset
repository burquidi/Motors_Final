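; AI controller for the Guardian that sets up its blackboard and behavior tree and relays patrol and attack commands to the pawn.
; On BeginPlay it stores the pawn's location as home and patrol points, writes the patrol and attack state enums, runs the tree and caches GuardianBP.
; Patrol and Attack events use cross-resetting DoOnce gates, so each pawn action fires only once per switch between the two.
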(event Custom|Patrol
  (bind _guardianbp (Variables|Default|GetGuardianBP))
  (Utilities|FlowControl|Sequence
    (:then_0
      (Utilities|FlowControl|DoOnce false
        (:Completed
          (Default|Patrol _guardianbp))))
    (:then_1
      (Utilities|FlowControl|DoOnce false) ; enters at Reset
    )))

(event Custom|Attack
  (bind _guardianbp (Variables|Default|GetGuardianBP))
  (Utilities|FlowControl|Sequence
    (:then_0
      (Utilities|FlowControl|DoOnce false
        (:Completed
          (Default|Attack _guardianbp))))
    (:then_1
      (Utilities|FlowControl|DoOnce false) ; enters at Reset
    )))

(event EventBeginPlay
  (bind _returnvalue (Pawn|GetControlledPawn))
  (bind _returnvalue_2 (Transformation|GetActorLocation _returnvalue))
  (bind _blackboardcomponent (Class|AIController|UseBlackboard "/Game/GuardianAI/AIGuardianBB.AIGuardianBB"))
  (AI|Components|Blackboard|SetValueasVector _blackboardcomponent (Utilities|Name|MakeLiteralName "HomeLocation") _returnvalue_2)
  (AI|Components|Blackboard|SetValueasVector _blackboardcomponent (Utilities|Name|MakeLiteralName "PatrolLocation") _returnvalue_2)
  (Utilities|FlowControl|Sequence
    (:then_0
      (AI|Components|Blackboard|SetValueasEnum _blackboardcomponent (Utilities|Name|MakeLiteralName "StatePatrol") (Utilities|Enum|LiteralenumEGuardianState "NewEnumerator0")))
    (:then_1
      (AI|Components|Blackboard|SetValueasEnum _blackboardcomponent (Utilities|Name|MakeLiteralName "StateAttack") (Utilities|Enum|LiteralenumEGuardianState "NewEnumerator1")))
    (:then_2
      (AI|RunBehaviorTree "/Game/GuardianAI/AIGuardianBT.AIGuardianBT")
      (Variables|Default|SetGuardianBP (.AsGuardian%20BP (Utilities|Casting|CastToGuardianBP (Pawn|GetControlledPawn)))))))

(fn ConstructionScript)