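; Guardian AI character that switches between Patrol and Attack states and drives its animation blueprint to match.
; Attack opens a gate and starts a self-repeating Melee loop with randomized punch and rest durations.
; Patrol closes the gate to end the loop, stops the melee animation and sets patrol.
; Left and right sphere overlaps deal heavy damage to any other actor, independent of state.
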(event Custom|Melee
  (Utilities|FlowControl|Gate true
    (:Exit
      (Default|Melee (Variables|Default|GetAnimInstance))
      (Utilities|FlowControl|Delay (Math|Random|RandomFloatinRange 2.0 8.0))
      (Default|StopMelee (Variables|Default|GetAnimInstance))
      (Utilities|FlowControl|Delay (Math|Random|RandomFloatinRange 2.0 4.0))
      (CallFunction|Melee))))

(event Custom|Patrol
  (bind _animinstance (Variables|Default|GetAnimInstance))
  (Utilities|FlowControl|Sequence
    (:then_0
      (Utilities|FlowControl|Gate true) ; enters at Close
    )
    (:then_1
      (Variables|Default|SetState "NewEnumerator0")
      (Default|StopMelee _animinstance)
      (Default|SetPatrol _animinstance))))

(event Custom|Attack
  (Variables|Default|SetState "NewEnumerator1")
  (Utilities|FlowControl|Sequence
    (:then_0
      (Utilities|FlowControl|Gate true) ; enters at Open
    )
    (:then_1
      (CallFunction|Melee))))

(event Custom|PunchEvent
  (params (OverlappedComponent :type Primitive%20Component%20Object%20Reference) (OtherActor :type Actor%20Object%20Reference) (OtherComp :type Primitive%20Component%20Object%20Reference) (OtherBodyIndex :type Integer) (bFromSweep :type Boolean) (SweepResult :type Hit%20Result%20Structure%20%28by%20ref%29))
  (if (!= OtherActor self)
    (Game|Damage|ApplyDamage OtherActor 1e+02 0 self)))

(event EventBeginPlay
  (Utilities|FlowControl|Sequence
    (:then_0
      (bind _asguardian_anim_bp (Utilities|Casting|CastToGuardianAnimBP (Components|SkeletalMesh|GetAnimInstance (Variables|Character|GetMesh))))
      (Variables|Default|SetAnimInstance _asguardian_anim_bp))
    (:then_1
      (Collision|BindEventtoOnComponentBeginOverlap (Variables|Default|GetSphereR) (delegate Custom|PunchEvent))
      (Collision|BindEventtoOnComponentBeginOverlap (Variables|Default|GetSphereL) (delegate Custom|PunchEvent)))))

(fn ConstructionScript)